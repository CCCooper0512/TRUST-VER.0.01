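; Movement component that handles walking, crouching and stamina-limited sprinting for the character passed to Initialize.
; Each state sets the character's max walk speed, and crouching also shortens or lengthens the capsule through L1_PlayerCharacter.
; Looping function-name timers drain SP while sprinting and moving, stopping at the minimum or standstill, and regenerate it after a retriggerable delay.
; SP changes are printed to screen for debugging.
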(event `StartCrouching`
  ;[1 1 1] Crunch
  (`KismetSystemLibrary.K2_ClearTimer` null "SprintTimer1")
  (`self.SetMaxWalkSpeed` (`self.CrouchSpeed`))
  (`/Game/GameBP/level1/L1_PlayerCharacter.ShortenPlayerCapsule` (cast `/Game/GameBP/level1/L1_PlayerCharacter` (`self.PlayerCharacter`) :!pure true))
  (set `self.IsCrunching?` true))

(event `StartSprint`
  ;[1 1 1] Sprint
  ;;[1 1 1] StartSprint
  (if (`self.IsCrunching?`)
    (`self.StopCrunching`))
  (if (and (> (`self.CurrentSP`) (`self.MinSP`)) (> (`KismetMathLibrary.VSize` (`Actor.GetVelocity` (`self.PlayerCharacter`))) 10.0))
    (`KismetSystemLibrary.K2_ClearTimer` null "RegenerateSp1")
    (`self.SetMaxWalkSpeed` (`self.SprintSpeed`))
    (`KismetSystemLibrary.K2_SetTimer` null "SprintTimer1" 0.1 true)))

(event `StopCrunching`
  ;[1 1 1] Crunch
  (`self.SetMaxWalkSpeed` (`self.WalkSpeed`))
  (`/Game/GameBP/level1/L1_PlayerCharacter.LengthenPlayerCapsule` (cast `/Game/GameBP/level1/L1_PlayerCharacter` (`self.PlayerCharacter`) :!pure true))
  (set `self.IsCrunching?` false))

(event `SprintTimer1`
  ;[1 1 1] Sprint
  ;;[1 1 1] SprintTimer
  (if (> (`KismetMathLibrary.VSize` (`Actor.GetVelocity` (`self.PlayerCharacter`))) 10.0)
    (bind _output_get (set `self.CurrentSP` (`KismetMathLibrary.FClamp` (- (`self.CurrentSP`) 1.0) (`self.MinSP`) (`self.MaxSP`))))
    (`KismetSystemLibrary.PrintString` (`KismetStringLibrary.Conv_DoubleToString` _output_get))
    (if (<= (`self.CurrentSP`) (`self.MinSP`))
      (`self.StopSprint`))
    (else
      (`self.StopSprint`))))

(event `StopSprint`
  ;[1 1 1] Sprint
  ;;[1 1 1] StopSprint
  (if (not (`self.IsCrunching?`))
    (`KismetSystemLibrary.K2_ClearTimer` null "SprintTimer1")
    (`self.SetMaxWalkSpeed` (`self.WalkSpeed`))
    (`KismetSystemLibrary.RetriggerableDelay` 5.0)
    (if (not (`KismetSystemLibrary.K2_IsTimerActive` null "SprintTimer1"))
      (`KismetSystemLibrary.PrintString` "GeneratingSP")
      (`KismetSystemLibrary.K2_SetTimer` null "RegenerateSp1" 0.3 true))))

(event `RegenerateSp1`
  ;[1 1 1] Sprint
  ;;[1 1 1] RegenerateSP
  (bind _output_get (set `self.CurrentSP` (`KismetMathLibrary.FClamp` (+ (`self.CurrentSP`) 1.0) (`self.MinSP`) (`self.MaxSP`))))
  (`KismetSystemLibrary.PrintString` (`KismetStringLibrary.Conv_DoubleToString` _output_get))
  (if (>= (`self.CurrentSP`) 100.0)
    (`KismetSystemLibrary.K2_ClearTimer` null "RegenerateSp1")
    (`KismetSystemLibrary.PrintString` "EndGeneratingSP")))

(fn `Initialize`
  (params (Character :type "Character Object Reference"))
  (set `self.PlayerCharacter` Character)
  (`self.SetMaxWalkSpeed` (`self.WalkSpeed`)))

(fn `SetMaxWalkSpeed`
  (params (`最大行走速度` :type "Float (single-precision)"))
  (set `CharacterMovementComponent.MaxWalkSpeed` `最大行走速度` (`Character.CharacterMovement` (`self.PlayerCharacter`))))